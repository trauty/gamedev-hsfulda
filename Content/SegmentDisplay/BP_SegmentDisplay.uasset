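; BP_SegmentDisplay is a numeric score display built from four child-actor digit segments.
; AddScore adds to a running score, then peels off decimal digits with modulo and integer division, from Segment4 to Segment1.
; Each digit goes to that child BP_Segment through SetDigit, so Segment4 shows the ones place.
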(event `AddScore`
  (params (Score :type Integer))
  (bind _output_get (set `self.Score` (+ Score (`self.Score`))))
  (bind _output_get_2 (set `self.TempScore` _output_get))
  (for _array_element (`|MakeArray` (`self.Segment4`) (`self.Segment3`) (`self.Segment2`) (`self.Segment1`))
    (bind _asbp_segment (cast `/Game/SegmentDisplay/BP_Segment` (`ChildActorComponent.ChildActor` _array_element)))
    (`/Game/SegmentDisplay/BP_Segment.SetDigit` _asbp_segment (mod _output_get_2 10))
    (set `self.TempScore` (/ _output_get_2 10))))

(fn `UserConstructionScript`)