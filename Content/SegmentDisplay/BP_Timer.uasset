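; Countdown timer actor that shows minutes, seconds and hundredths on six BP_Segment child-actor digit displays.
; BeginPlay combines Minutes, Seconds and Milliseconds into TotalSeconds, weighted by 3600, 60 and 1.
; Tick subtracts game time from that total and splits the remainder into digits by powers of ten, using nested loops over segment pairs.
; Below zero, it clears IsRunning if set and plays a finish sound at the actor.
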(event `self.ReceiveBeginPlay`
  (set `self.TotalSeconds` (+ (* (`self.Minutes`) 3600) (* (`self.Seconds`) 60) (`self.Milliseconds`))))

(event `self.ReceiveTick`
  (params (DeltaSeconds :type "Float (single-precision)"))
  (bind _returnvalue (- (`self.TotalSeconds`) (`KismetSystemLibrary.GetGameTimeInSeconds`)))
  (if (>= _returnvalue 0.0)
    (for (_array_element _array_index) (`|MakeArray` (`self.BP_Segment2`) (`self.BP_Segment3`))
      (bind _asbp_segment (cast `/Game/SegmentDisplay/BP_Segment` (`ChildActorComponent.ChildActor` _array_element)))
      (`/Game/SegmentDisplay/BP_Segment.SetDigit` _asbp_segment (mod (/ (mod (`KismetMathLibrary.FTrunc` _returnvalue) 60) (`KismetMathLibrary.FTrunc` (`KismetMathLibrary.MultiplyMultiply_FloatFloat` 10.0 (`KismetMathLibrary.Conv_IntToDouble` _array_index)))) 10))
      (for (_array_element_2 _array_index_2) (`|MakeArray` (`self.BP_Segment`) (`self.BP_Segment1`))
        (bind _asbp_segment_2 (cast `/Game/SegmentDisplay/BP_Segment` (`ChildActorComponent.ChildActor` _array_element_2)))
        (`/Game/SegmentDisplay/BP_Segment.SetDigit` _asbp_segment_2 (mod (/ (* (`KismetMathLibrary.FMod` _returnvalue 1.0) 100.0) (`KismetMathLibrary.FTrunc` (`KismetMathLibrary.MultiplyMultiply_FloatFloat` 10.0 (`KismetMathLibrary.Conv_IntToDouble` _array_index_2)))) 10))
        (for (_array_element_3 _array_index_3) (`|MakeArray` (`self.BP_Segment4`) (`self.BP_Segment5`))
          (bind _asbp_segment_3 (cast `/Game/SegmentDisplay/BP_Segment` (`ChildActorComponent.ChildActor` _array_element_3)))
          (`/Game/SegmentDisplay/BP_Segment.SetDigit` _asbp_segment_3 (mod (/ (/ _returnvalue 60.0) (`KismetMathLibrary.FTrunc` (`KismetMathLibrary.MultiplyMultiply_FloatFloat` 10.0 (`KismetMathLibrary.Conv_IntToDouble` _array_index_3)))) 10)))))
    (elif (`self.IsRunning`)
      (set `self.IsRunning` false)
      (`self.OnTimerFinished`))))

(event `OnTimerFinished`
  (`GameplayStatics.PlaySoundAtLocation` "/Game/SegmentDisplay/A_FinishSound.A_FinishSound" (`self.K2_GetActorLocation`) (struct) 1.0 1.0 0.0 null null null null))

(fn `UserConstructionScript`)