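; BP_CustomGameMode is a game mode that tracks the score and runs a countdown timer.
; AddScore adds to a clamped total and broadcasts the new value through OnScoreChanged.
; BeginPlay converts the configured minutes and seconds into a time limit.
; Tick broadcasts the time left against elapsed game time through OnTimeChanged, then clears IsTimerRunning and plays a finish sound once if the timer was running.
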(event `AddScore`
  (params (Score :type Integer))
  (bind _output_get (set `self.TotalScore` (`KismetMathLibrary.Clamp` (+ Score (`self.TotalScore`)) 0 9999)))
  (`self.OnScoreChanged` _output_get))

(event `self.ReceiveBeginPlay`
  (set `self.TotalSeconds` (+ (* (`self.Minutes`) 60) (`self.Seconds`))))

(event `self.ReceiveTick`
  (params (DeltaSeconds :type "Float (single-precision)"))
  (bind _returnvalue (- (`self.TotalSeconds`) (`KismetSystemLibrary.GetGameTimeInSeconds`)))
  (if (>= _returnvalue 0.0)
    (`self.OnTimeChanged` _returnvalue)
    (elif (`self.bIsTimerRunning`)
      (set `self.bIsTimerRunning` false)
      (`GameplayStatics.PlaySound2D` "/Game/SegmentDisplay/A_FinishSound.A_FinishSound" 1.0 1.0 0.0 null null))))

(fn `UserConstructionScript`)