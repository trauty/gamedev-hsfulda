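; BP_Target is a swaying shootable target that awards points to BP_CustomGameMode when destroyed.
; Tick offsets it from its starting location along its right and up vectors using cosine and sine of game time, scaled by SwaySpeed and SwayRange.
; OnShotHit plays a sound, then zeroes Health, adds score and destroys the actor only if Damage minus Health is zero or less.
; Health is never decremented, so larger hits leave it intact.
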(event `self.ReceiveBeginPlay`
  (set `self.StartLocation` (`self.K2_GetActorLocation`)))

(event `/Game/BPI_Shootable.OnShotHit`
  (params (Damage :type Integer))
  (`GameplayStatics.PlaySoundAtLocation` "/Game/Items/A_Pickup.A_Pickup" (`self.K2_GetActorLocation`) (struct) 1.0 1.0 0.0 null null null null)
  (if (<= (- Damage (`self.Health`)) 0)
    (set `self.Health` 0)
    (bind _asbp_custom_game_mode (cast `/Game/BP_CustomGameMode` (`GameplayStatics.GetGameMode`)))
    (`/Game/BP_CustomGameMode.AddScore` _asbp_custom_game_mode (`self.Points`))
    (`self.K2_DestroyActor`)))

(event `self.ReceiveTick`
  (params (DeltaSeconds :type "Float (single-precision)"))
  (bind (_swayrange_x _swayrange_y) (`KismetMathLibrary.BreakVector` (`self.SwayRange`)))
  (bind (_swayrange_x_2 _swayrange_y_2 _swayrange_z) (`KismetMathLibrary.BreakVector` (`self.SwayRange`)))
  (bind _returnvalue (* (`KismetSystemLibrary.GetGameTimeInSeconds`) (`self.SwaySpeed`)))
  (`self.K2_SetActorLocation` (+ (* (* (`KismetMathLibrary.Sin` _returnvalue) _swayrange_z) (`self.GetActorUpVector`)) (* (* (`KismetMathLibrary.Cos` _returnvalue) _swayrange_y) (`self.GetActorRightVector`)) (`self.StartLocation`))))

(fn `UserConstructionScript`)