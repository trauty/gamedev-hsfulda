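; BP_Item is a collectible pickup that awards points and destroys itself when any actor overlaps it.
; On overlap it prints the points, plays a metal pipe sound and passes the score to DisplayRef.
; Tick adds time-based cosine and sine offsets to its current location, producing a frame-rate-dependent looping motion in the XZ plane.
; The construction script slightly randomizes its uniform scale.
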(event `self.ReceiveActorBeginOverlap`
  (params (OtherActor :type "Actor Object Reference"))
  (`KismetSystemLibrary.PrintString` (`KismetStringLibrary.Concat_StrStr` "Eingesammelt: " (`KismetStringLibrary.Conv_IntToString` (`self.Points`))))
  (`GameplayStatics.PlaySoundAtLocation` "/Game/Items/A_VoicMetalPipe.A_VoicMetalPipe" (`self.K2_GetActorLocation`) (struct) 1.0 1.0 0.0 null null null null)
  (`/Game/SegmentDisplay/BP_SegmentDisplay.AddScore` (`self.DisplayRef`) (`self.Points`))
  (`self.K2_DestroyActor`))

(event `self.ReceiveTick`
  (params (DeltaSeconds :type "Float (single-precision)"))
  (bind _rotationscale (`self.RotationScale`))
  (bind _returnvalue (* (`KismetSystemLibrary.GetGameTimeInSeconds`) (`self.MovementSpeed`)))
  (`self.K2_SetActorRelativeLocation` (+ (`self.K2_GetActorLocation`) (`KismetMathLibrary.MakeVector` (* _rotationscale (`KismetMathLibrary.Cos` _returnvalue)) 0.0 (* (`KismetMathLibrary.Sin` _returnvalue) _rotationscale)))))

(fn `UserConstructionScript`
  (`self.SetActorScale3D` (`KismetMathLibrary.Conv_DoubleToVector` (+ (* (`KismetMathLibrary.RandomFloat`) 0.2) 1.0))))