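; BP_Segment is a seven-segment display that shows a digit by lighting its segment components A to G.
; SetDigit looks up the digit's on/off pattern in the Segments table and sets each component's EmissionStrength material parameter to the configured strength or zero.
; The construction script calls SetDigit, and BeginPlay repeats the same logic inline to apply the initial digit at runtime.
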(event `self.ReceiveBeginPlay`
  (bind (_a _b _c _d _e _f _g) (break `/Game/Items/S_Segments` (`|GetArrayItem` (`self.Segments`) (`self.Digit`))))
  (bind _output_get (set `self.Array` (`|MakeArray` (`self.A`) (`self.B`) (`self.C`) (`self.D`) (`self.E`) (`self.F`) (`self.G`))))
  (for (_array_element _array_index) _output_get
    (`MeshComponent.SetScalarParameterValueOnMaterials` _array_element "EmissionStrength" (`KismetMathLibrary.SelectFloat` (`self.EmissionStrength`) 0.0 (`|GetArrayItem` (`|MakeArray` _a _b _c _d _e _f _g) _array_index)))))

(fn `SetDigit`
  (params (Digit :type Integer))
  (bind (_a _b _c _d _e _f _g) (break `/Game/Items/S_Segments` (`|GetArrayItem` (`self.Segments`) Digit)))
  (for (_array_element _array_index) (`self.Array`)
    (`MeshComponent.SetScalarParameterValueOnMaterials` _array_element "EmissionStrength" (`KismetMathLibrary.SelectFloat` (`self.EmissionStrength`) 0.0 (`|GetArrayItem` (`|MakeArray` _a _b _c _d _e _f _g) _array_index)))))

(fn `UserConstructionScript`
  (set `self.Array` (`|MakeArray` (`self.A`) (`self.B`) (`self.C`) (`self.D`) (`self.E`) (`self.F`) (`self.G`)))
  (`self.SetDigit` (`self.Digit`)))